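; BP_Player is the player Blueprint, handling the stat HUD, shot effects and damage scoring.
; On BeginPlay, only a locally controlled instance creates the stat HUD widget and adds it to the viewport.
; MuzzleFlash attaches an explosion emitter at the muzzle, while HitLocation re-traces the supplied hit on Visibility to spawn one just off the surface.
; OnDamageDone adds truncated damage to the DamageDone score.
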(event EventBeginPlay
  (if (Pawn|IsLocallyControlled)
    (bind _returnvalue (UserInterface|CreateWidget "/Game/WBP_StatHud.WBP_StatHud_C"))
    (Utilities|IsValid _returnvalue
      (:Is%20Valid
        (UserInterface|Viewport|AddtoViewport _returnvalue 0)))))

(event Collision|EventActorBeginOverlap
  (params (OtherActor :type Actor%20Object%20Reference)))

(event EventTick
  (params (DeltaSeconds :type Float%20%28single-precision%29)))

(event EventMuzzleFlash
  (Effects|SpawnEmitterAttached "/Game/StarterContent/Particles/P_Explosion.P_Explosion" (Variables|Default|GetMuzzleLocation) "None" "0, 0, 0" "0, 0, 0" (Variables|Default|GetsizeOffFlash)))

(event EventHitLocation
  (params (hit :type Hit%20Result%20Structure))
  (bind (_outhit _returnvalue) (Collision|LineTraceByChannel (.tracestart hit) (.traceend hit) "TraceTypeQuery1" false 0 "None"))
  (if _returnvalue
    (Effects|SpawnEmitteratLocation "/Game/StarterContent/Particles/P_Explosion.P_Explosion" (+ (.impactpoint _outhit) (* (.normal _outhit) 2.0)) "0, 0, 0" (Variables|Default|GetsizeOffFlash))))

(event EventOnDamageDone
  (params (Value :type Float%20%28single-precision%29))
  (Class|FGnetworkProjScoreComponent|AddScore (Variables|Default|GetFGnetworkProjScore) "DamageDone" (Math|Float|Truncate Value)))

(fn ConstructionScript)